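; Tank Blueprint that lets the player orbit the camera with the arrow keys, with no other gameplay logic in its graphs.
; The InputSetup graph feeds azimuth axis inputs into AzimuthGimble as local yaw and elevation inputs into SpringArm as local pitch, separating the two rotation axes.
; Axis values are applied directly as rotation deltas, without delta-time scaling or clamping.
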(event EventBeginPlay)

(event Collision|EventActorBeginOverlap
  (params (OtherActor :type Actor%20Object%20Reference)))

(event EventTick
  (params (DeltaSeconds :type Float%20%28single-precision%29)))

(event Input|AxisEvents|InputAxisAimAzimuthRight
  (params (AxisValue :type Float%20%28single-precision%29))
  ;[1 1 1] Input Binding for Left and Right Camera With Arrow Keys
  (Transformation|AddLocalRotation (Variables|Default|GetAzimuth%20Gimble) (Math|Rotator|MakeRotator 0.0 0.0 AxisValue) false false))

(event Input|AxisEvents|InputAxisAimElevationUp
  (params (AxisValue :type Float%20%28single-precision%29))
  ;[1 1 1] Input Binding For Up And Down Camera With Arrow Keys
  (Transformation|AddLocalRotation (Variables|Default|GetSpringArm) (Math|Rotator|MakeRotator 0.0 AxisValue 0.0) false false))

(event Input|AxisEvents|InputAxisAimElevationDown
  (params (AxisValue :type Float%20%28single-precision%29))
  ;[1 1 1] Input Binding For Up And Down Camera With Arrow Keys
  (bind _result (Math|Float|NegateFloat AxisValue)
    (:%20%20
      (Transformation|AddLocalRotation (Variables|Default|GetSpringArm) (Math|Rotator|MakeRotator 0.0 _result 0.0) false false))))

(event Input|AxisEvents|InputAxisAimAzimuthLeft
  (params (AxisValue :type Float%20%28single-precision%29))
  ;[1 1 1] Input Binding for Left and Right Camera With Arrow Keys
  (bind _result (Math|Float|NegateFloat AxisValue)
    (:%20%20
      (Transformation|AddLocalRotation (Variables|Default|GetAzimuth%20Gimble) (Math|Rotator|MakeRotator 0.0 0.0 _result) false false))))

(fn ConstructionScript)